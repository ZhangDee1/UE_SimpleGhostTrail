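; BPC_GhostTrail is an actor component that links its owner's skeletal mesh to the BP_GhostTrailManager actor that handles ghost trail spawning.
; On BeginPlay it caches the mesh and the manager found in the level, then calls InitManager with that mesh.
; Its anim notify events call InitManager again to activate and DeactivateSpawn to stop, guarded by validity checks.
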(event Custom|ActivateByAnimNotify
  ;[1 1 1] 动画通知开始
  (if (and (Utilities|IsValid (Variables|Default|GetGhostManager)) (Utilities|IsValid (Variables|Default|GetOwningSkeletal)))
    (Default|InitManager (Variables|Default|GetGhostManager) (Variables|Default|GetOwningSkeletal))))

(event Custom|DeactivateByAnimNotify
  ;[1 1 1] 动画通知开始
  (if (and (Utilities|IsValid (Variables|Default|GetGhostManager)) (Utilities|IsValid (Variables|Default|GetOwningSkeletal)))
    (Default|DeactivateSpawn (Variables|Default|GetGhostManager))))

(event EventBeginPlay
  (bind _returnvalue (Components|GetOwner))
  (bind _returnvalue_2 (Actor|GetComponentbyClass _returnvalue "/Script/Engine.SkeletalMeshComponent"))
  ;[1 1 1] Init
  (if (and (Utilities|IsValid _returnvalue) (Utilities|IsValid _returnvalue_2))
    (Variables|Default|SetOwningSkeletal _returnvalue_2)
    (bind _returnvalue_3 (Actor|GetActorOfClass "/Game/GhostTrail/BP_GhostTrailManager.BP_GhostTrailManager_C"))
    (Variables|Default|SetGhostManager _returnvalue_3)
    (Default|InitManager _returnvalue_3 (Variables|Default|GetOwningSkeletal))))