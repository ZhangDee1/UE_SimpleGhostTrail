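; Ghost trail manager that leaves timed afterimages of a skeletal mesh, handed to it by BPC_GhostTrail through InitManager.
; While the spawn flag is on, Tick periodically adds a PoseableMesh component that snapshots the target's transform, mesh and pose.
; All ghosts share one dynamic ghost material instance.
; Tick also counts down each ghost's life and destroys expired ones, even after DeactivateSpawn stops new spawns.
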(event Custom|InitManager
  (params (TargetSkeleton :type Skeletal%20Mesh%20Component%20Object%20Reference))
  (Variables|Default|SetTargetSkeleton TargetSkeleton))

(event Custom|DeactivateSpawn
  (Variables|配置|Set激活残影 false))

(event EventTick
  (params (DeltaSeconds :type Float%20%28single-precision%29))
  (CallFunction|UpdateGhostTimer)
  (if (Variables|配置|Get激活残影)
    (bind _output_get (Variables|Default|SetGhostSpawnTimer (+ (Variables|Default|GetGhostSpawnTimer) DeltaSeconds)))
    (if (>= _output_get (Variables|配置|Get生成间隔))
      (CallFunction|SpawnGhosts)
      (Variables|Default|SetGhostSpawnTimer 0.0))))

(event EventBeginPlay
  ;[1 1 1] Creater Dynamic Mat
  (Utilities|IsValid (Variables|配置|Get幽灵材质)
    (:Is%20Valid
      (bind _returnvalue (Rendering|Material|CreateDynamicMaterialInstance (Variables|配置|Get幽灵材质) "None" "None" :!class /Script/Engine.KismetMaterialLibrary))
      (Variables|Default|SetDynamicMat _returnvalue))))

(fn ConstructionScript)

(fn SpawnGhosts
  (Utilities|IsValid (Variables|Default|GetTargetSkeleton) ; 多判断一下防止出错
    (:Is%20Valid
      (Utilities|FlowControl|Sequence
        (:then_0
          (bind _returnvalue (AddComponent|AddPoseableMeshComponent false))
          (bind _output_get (LocalVariables|SetLocalSKMesh _returnvalue))
          (Transformation|SetWorldTransform _output_get (Transformation|GetWorldTransform (Variables|Default|GetTargetSkeleton)) false false))
        (:then_1
          (Class|SkinnedMeshComponent|SetSkeletalMesh (LocalVariables|GetLocalSKMesh) (Variables|/Script/Engine.SkinnedMeshComponent|GetSkeletalMesh (Variables|Default|GetTargetSkeleton)) true)
          (Utilities|IsValid (Variables|Default|GetDynamicMat)
            (:Is%20Valid
              _)
            (:Is%20Not%20Valid
              (bind _returnvalue_2 (Rendering|Material|CreateDynamicMaterialInstance (Variables|配置|Get幽灵材质) "None" "None" :!class /Script/Engine.KismetMaterialLibrary))
              (Variables|Default|SetDynamicMat _returnvalue_2)))
          (for _index (range 0 (- (Rendering|Material|GetNumMaterials (Variables|Default|GetTargetSkeleton)) 1))
            (Rendering|Material|SetMaterial (LocalVariables|GetLocalSKMesh) _index (Variables|Default|GetDynamicMat))))
        (:then_2
          (Class|PoseableMeshComponent|CopyPosefromSkeletalComponent (LocalVariables|GetLocalSKMesh) (Variables|Default|GetTargetSkeleton))
          (Utilities|Array|Add (Variables|Default|GetGhosts) (Utilities|Struct|MakeFGhostTrial (LocalVariables|GetLocalSKMesh) (Variables|配置|Get幽灵自动销毁时间))))))))

(fn UpdateGhostTimer
  (bind _ghosts (Variables|Default|GetGhosts))
  (if (> (Utilities|Array|Length (Variables|Default|GetGhosts)) 0)
    (for (_ _array_index) _ghosts
      (if (<= (- (.Life (Utilities|Struct|BreakFGhostTrial (Utilities|Array|Get(acopy) _ghosts _array_index))) (Utilities|Time|GetWorldDeltaSeconds)) 0.0)
        (Components|DestroyComponent (.Mesh (Utilities|Struct|BreakFGhostTrial (Utilities|Array|Get(acopy) _ghosts _array_index))))
        (Utilities|Array|RemoveIndex (Variables|Default|GetGhosts) _array_index)
        (else
          (Utilities|Struct|SetmembersinFGhostTrial (Utilities|Array|Get(acopy) _ghosts _array_index) (- (.Life (Utilities|Struct|BreakFGhostTrial (Utilities|Array|Get(acopy) _ghosts _array_index))) (Utilities|Time|GetWorldDeltaSeconds))))))))